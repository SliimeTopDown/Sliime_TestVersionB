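; Player character Blueprint with a sprite, handling movement input and a forward probe trace.
; IA_Move waits on a 0.2-second Delay, then feeds the action's X and Y into movement input along world X and Y.
; Every Tick, a Visibility line trace runs from the sprite along its forward vector for LineTraceLength, drawn for debugging.
; The trace result is not used.
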(event `EnhancedInput|/Game/BluePaper/Controler/input/IA_Move`
  (params (ActionValue :type "Vector2D Structure") (ElapsedSeconds :type "Float (double-precision)") (TriggeredSeconds :type "Float (double-precision)") (InputAction :type "InputAction Object Reference" :default "/Game/BluePaper/Controler/input/IA_Move.IA_Move"))
  (bind (_x _y) (`KismetMathLibrary.BreakVector2D` ActionValue))
  (:`Triggered`
    (`KismetSystemLibrary.Delay` 0.2)
    (set `self.X` _x)
    (set `self.Y` _y)
    (`self.AddMovementInput` (1.0 0.0 0.0) (`self.X`))
    (`self.AddMovementInput` (0.0 1.0 0.0) (`self.Y`))))

(event `self.ReceiveBeginPlay`)

(event `self.ReceiveTick`
  (params (DeltaSeconds :type "Float (single-precision)"))
  (bind _sprite (`self.Sprite`))
  (bind _returnvalue (`SceneComponent.K2_GetComponentLocation` _sprite))
  (`KismetSystemLibrary.LineTraceSingle` :`Start` _returnvalue :`End` (+ _returnvalue (* (`SceneComponent.GetForwardVector` _sprite) (`self.LineTrace_Length`))) :`TraceChannel` "TraceTypeQuery1" :`DrawDebugType` "ForOneFrame"))

(fn `UserConstructionScript`)